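; BP_GridLines is an unfinished tile grid Blueprint meant to draw grid lines and support tile selection.
; Its construction script builds line and selection dynamic instances of M_Block, then loops over GridX to pass tile-spaced line endpoints and vertex/triangle arrays to CreateLine, printing debug text.
; CreateLine, tile conversion, selection and validity checks are stubs, and only one line direction is looped.
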(fn ConstructionScript
  (bind _materialinstance (Private|CreateMaterialInstance (Variables|Constants|GetLineColour) (Variables|Constants|GetLineOpacity)))
  (LocalVariables|SetLineMaterialInst _materialinstance)
  (bind _materialinstance_2 (Private|CreateMaterialInstance (Variables|Constants|GetSelectionColout) (Variables|Constants|GetSelectionOpacity)))
  (LocalVariables|SetSelectionMaterialInst _materialinstance_2)
  (Utilities|FlowControl|Sequence
    (:then_0
      (for _index (range 0 (Variables|Constants|GetGridX))
        (LocalVariables|SetLineStart (* _index (Variables|Constants|GetTileSize)))
        (bind _gridwidth (Private|GridWidth))
        (LocalVariables|SetLineEnd _gridwidth)
        (Private|CreateLine (Math|Vector|MakeVector (LocalVariables|GetLineStart) 0.0 0.0) (Math|Vector|MakeVector (LocalVariables|GetLineStart) (LocalVariables|GetLineEnd) 0.0) (Variables|Constants|GetLineThickness) (LocalVariables|GetLineVerticies) (LocalVariables|GetLineTriangles))
        (Development|PrintString "Hello")))))

(fn CreateLine
  (params (Start :type Vector) (End :type Vector) (Thickness :type Float%20%28double-precision%29) (Vertecies :type Array%20of%20Vectors) (Triangles :type Array%20of%20Integers)))

(fn GridWidth
  (return (* (Variables|Constants|GetGridY) (Variables|Constants|GetTileSize))))

(fn GridHeight
  (return (* (Variables|Constants|GetGridX) (Variables|Constants|GetTileSize))))

(fn CreateMaterialInstance
  (params (Colour :type Linear%20Color%20Structure) (Opacity :type Float%20%28double-precision%29))
  (bind _returnvalue (Rendering|Material|CreateDynamicMaterialInstance "/Game/Blueprint/M_Block.M_Block" "None" "None" :!class /Script/Engine.KismetMaterialLibrary))
  (Rendering|Material|SetVectorParameterValue _returnvalue "Colour" Colour :!class /Script/Engine.MaterialInstanceDynamic)
  (Rendering|Material|SetScalarParameterValue _returnvalue "Opacity" Opacity :!class /Script/Engine.MaterialInstanceDynamic)
  (return _returnvalue))

(fn LocationtoTile
  (params (Location :type Vector))
  (return false 0 0))

(fn TiletoGridLocation
  (params (X :type Integer) (Y :type Integer) (IsCenter :type Boolean))
  (return false ""))

(fn SetSelectedTile
  (params (X :type Integer) (Y :type Integer)))