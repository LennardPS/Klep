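; Default player pawn that acts as a camera rig with pan, zoom and cursor picking through Enhanced Input.
; It registers its mapping context on BeginPlay, and zoom input drives a clamped spring arm length.
; Hold sets a flag that lets pointer input slide the root across world XY, with Y inverted and scaled by sensitivity.
; Tap and hold trace under the cursor on separate channels, currently only printing the hit actor's name.
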(event Input|EnhancedActionEvents|EnhancedInputActionInputAction_Zoom
  (params (ActionValue :type Float%20%28double-precision%29) (ElapsedSeconds :type Float%20%28double-precision%29) (TriggeredSeconds :type Float%20%28double-precision%29) (InputAction :type Input%20Action%20Object%20Reference :default "/Game/Blueprint/Inputs/InputAction_Zoom.InputAction_Zoom"))
  ;[1 1 1] Zoom
  (:Triggered
    (bind _output_get (Variables|Default|SetZoomDistance (Math|Float|Clamp(Float) (+ (* ActionValue (.z (Variables|Default|GetCameraMovementSensitivity))) (Variables|Default|GetZoomDistance)) 2.5e+02 7.5e+02)))
    (Variables|/Script/Engine.SpringArmComponent|SetTargetArmLength (Variables|Default|GetSpringArm) _output_get)))

(event Input|EnhancedActionEvents|EnhancedInputActionInputAction_Hold
  (params (ActionValue :type Boolean) (ElapsedSeconds :type Float%20%28double-precision%29) (TriggeredSeconds :type Float%20%28double-precision%29) (InputAction :type Input%20Action%20Object%20Reference :default "/Game/Blueprint/Inputs/InputAction_Hold.InputAction_Hold"))
  (bind _returnvalue (Game|GetPlayerController 0))
  (bind (_hitresult _returnvalue_2) (Game|Player|GetHitResultUnderCursorbyChannel _returnvalue "TraceTypeQuery4" true))
  (:Triggered
    (Variables|Default|SetIsHeld ActionValue)
    (if _returnvalue_2
      (if (Variables|Default|GetIsHeld)
        (Development|PrintString (Utilities|GetDisplayName (.hitactor _hitresult)))))))

(event Input|EnhancedActionEvents|EnhancedInputActionInputAction_PointerPosition
  (params (ActionValue :type Vector%202D%20Structure) (ElapsedSeconds :type Float%20%28double-precision%29) (TriggeredSeconds :type Float%20%28double-precision%29) (InputAction :type Input%20Action%20Object%20Reference :default "/Game/Blueprint/Inputs/InputAction_PointerPosition.InputAction_PointerPosition"))
  (bind _defaultsceneroot (Variables|Default|GetDefaultSceneRoot))
  (bind _returnvalue (Transformation|GetWorldLocation _defaultsceneroot))
  ;[1 1 1] Pointer Position
  (:Triggered
    (Variables|Default|SetPointerPosition ActionValue)
    (if (Variables|Default|GetIsHeld)
      (Transformation|SetWorldLocation _defaultsceneroot (Math|Vector|MakeVector (+ (.x (* (Variables|Default|GetPointerPosition) (Variables|Default|GetCameraMovementSensitivity))) (.x _returnvalue) 0.0) (+ (* (.y (* (Variables|Default|GetPointerPosition) (Variables|Default|GetCameraMovementSensitivity))) -1.0) (.y _returnvalue)) (.z _returnvalue)) false false))))

(event Input|EnhancedActionEvents|EnhancedInputActionInputAction_Tap
  (params (ActionValue :type Boolean) (ElapsedSeconds :type Float%20%28double-precision%29) (TriggeredSeconds :type Float%20%28double-precision%29) (InputAction :type Input%20Action%20Object%20Reference :default "/Game/Blueprint/Inputs/InputAction_Tap.InputAction_Tap"))
  (bind _returnvalue (Game|GetPlayerController 0))
  (bind (_hitresult _returnvalue_2) (Game|Player|GetHitResultUnderCursorbyChannel _returnvalue "TraceTypeQuery3" true))
  (:Triggered
    (if _returnvalue_2
      (Development|PrintString (Utilities|GetDisplayName (.hitactor _hitresult)) true true "(R=1.000000,G=0.000000,B=0.028754,A=1.000000)"))))

(event EventBeginPlay
  (bind _asplayer_controller_default (Utilities|Casting|CastToPlayerController_Default (Pawn|GetController)))
  (Utilities|IsValid (PlayerController|LocalPlayerSubsystems|GetEnhancedInputLocalPlayerSubsystem _asplayer_controller_default)
    (:Is%20Valid
      (Input|AddMappingContext (PlayerController|LocalPlayerSubsystems|GetEnhancedInputLocalPlayerSubsystem _asplayer_controller_default) "/Game/Blueprint/Inputs/InputMappingContext_Default.InputMappingContext_Default" 0 "(bIgnoreAllPressedKeysUntilRelease=True,bForceImmediately=False)"))))

(fn ConstructionScript)