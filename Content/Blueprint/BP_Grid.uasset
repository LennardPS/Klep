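; BP_Grid is an actor that fills a configurable X by Y grid with small, randomly rotated cone meshes.
; Its construction script uses nested loops over GridX and GridY, spacing positions by TileSize and printing a debug string inside the inner loop.
; Func_SpawnMesh adds a scaled-down static mesh component at each position.
; An alternative that spawns BP_Block child actors remains in that function but never runs.
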(fn ConstructionScript
  (bind _tilesize (Variables|Default|GetTileSize))
  (Utilities|FlowControl|Sequence
    (:then_0
      (for _index (range 0 (- (Variables|Default|GetGridX) 1))
        (CallFunction|FuncSpawnMesh (Math|Vector|MakeVector (* _index (Variables|Default|GetTileSize)) 0.0 0.0))
        (for _index_2 (range 0 (- (Variables|Default|GetGridY) 2))
          (CallFunction|FuncSpawnMesh (Math|Vector|MakeVector (* _index (Variables|Default|GetTileSize)) (+ (* _index_2 _tilesize) _tilesize) 0.0))
          (Development|PrintString "Hello"))))))

(fn FuncSpawnMesh
  (params (Spawn%20Transform%20Location :type Vector))
  (bind _returnvalue (AddComponent|AddStaticMeshComponent false (Math|Transform|MakeTransform Spawn%20Transform%20Location (Math|Random|RandomRotator false) "0.200000,0.200000,0.200000")))
  (Components|StaticMesh|SetStaticMesh _returnvalue "/Game/StarterContent/Shapes/Shape_Cone.Shape_Cone"))